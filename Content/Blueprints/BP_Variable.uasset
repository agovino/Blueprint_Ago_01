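; BP_Variable is a practice Blueprint that demonstrates variable types, including boolean, integer, float, vector and object reference, by printing them on screen.
; On BeginPlay it branches on TestBoolean and prints True or False, while the construction script sets TestVector.
; Disconnected snippets, some in separate Integer and Float Addition graphs, show validity checks, value-to-string printing, a for loop and int-to-float addition, but never execute.
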(event EventBeginPlay
  (if (Variables|Default|GetTestBoolean)
    (Development|PrintString "True")
    (else
      (Development|PrintString "False"))))

(event EventTick
  (params (DeltaSeconds :type Float%20%28single-precision%29)))

(fn ConstructionScript
  (Variables|Default|SetTestVector "1.000000,2.000000,3.000000"))
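; BP_Character is a test Blueprint that repeats one debug-print routine as a custom event, a function and a macro.
; Each version checks CanPrint, then uses a loop to print a label naming its kind.
; Only the macro runs, from BeginPlay, and its exit is wired inside the loop body.
; The calls to the event and function are unconnected, and TestEvent is an empty graph.
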(event Custom|TestEvents
  (if (Variables|Default|GetbCanPrint)
    (for _index (range 0 4)
      (Development|PrintString "Event"))))

(event Collision|EventActorBeginOverlap
  (params (OtherActor :type Actor%20Object%20Reference)))

(event EventTick
  (params (DeltaSeconds :type Float%20%28single-precision%29)))

(event EventBeginPlay
  (Utilities|TestMacro))

(fn ConstructionScript)

(fn TestFunction
  (if (Variables|Default|GetbCanPrint)
    (for _index (range 0 4)
      (Development|PrintString "Function"))))

(fn TestEvent)